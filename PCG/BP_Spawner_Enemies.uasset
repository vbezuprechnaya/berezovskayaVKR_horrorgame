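; BP_Spawner_Enemies is a spawner actor that scatters chaser and warrior enemies around itself when play begins.
; BeginPlay runs SpawnChaser, which spawns BP_AI, then SpawnWarrior with MaxQuantity, whose spawn node shows no class.
; Each loop places actors at random reachable navigation points within a fixed radius of the spawner.
; Separate counters use inclusive comparisons, so counts starting at zero yield one spawn beyond the limit.
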(event Custom|SpawnChaser
  (while (<= (Variables|Default|GetCurrQuantity) (Variables|Default|GetMaxQuantity))
    (Math|Integer|IncrementInt (Variables|Default|GetCurrQuantity)
      (:%20%20
        (Game|SpawnActorfromClass "/Game/Enemies/Chaser/BP_AI.BP_AI_C" (Math|Transform|MakeTransform (.RandomLocation (AI|Navigation|GetRandomReachablePointinRadius (Transformation|GetActorLocation) 8e+03 0 0)) "0, 0, 0" "1.000000,1.000000,1.000000") "Undefined" "MultiplyWithRoot" 0 0)))))

(event Custom|SpawnWarrior
  (params (Amount :type Integer))
  (while (<= (Variables|Default|GetCurrentWarrirQuant) Amount)
    (Math|Integer|IncrementInt (Variables|Default|GetCurrentWarrirQuant)
      (:%20%20
        (Game|SpawnActorfromClass "/Game/Enemies/Warrior/BP_AIWarrior.BP_AIWarrior_C" (Math|Transform|MakeTransform (.RandomLocation (AI|Navigation|GetRandomReachablePointinRadius (Transformation|GetActorLocation) 8e+03 0 0)) "0, 0, 0" "1.000000,1.000000,1.000000") "Undefined" "MultiplyWithRoot" 0 0)))))

(event EventBeginPlay
  (CallFunction|SpawnChaser)
  (CallFunction|SpawnWarrior (Variables|Default|GetMaxQuantity)))

(fn ConstructionScript)