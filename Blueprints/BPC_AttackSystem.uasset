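; Attack component for BP_MainCharacter that plays sword, stab and kick montages and applies melee damage to "Damagable" actors.
; Combo input advances through four attacks via AttackIndex, with SaveAttack buffering input for SwordAttackCombo to continue or reset.
; Direct attack, stab and kick inputs play their montage and run a one-shot sphere trace.
; StartSwordTrace and StopSwordTrace control a looping timer tracing between sword points, with throttled damage.
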(event Custom|SwordAttack
  ;[0 0 0] Combo system
  ;;[0 0 0 0] Sword Attack
  (if (Variables|Default|GetIsAttacking)
    (Variables|Default|SetsaveAttack true)
    (else
      (Variables|Default|SetsaveAttack false)
      (switch int (Variables|Default|GetAttackIndex)
        (:0
          (CallFunction|Attack1))
        (:1
          (CallFunction|Attack2))
        (:2
          (CallFunction|Attack3))
        (:3
          (CallFunction|Attack4))))))

(event Custom|SwordAttackCombo
  ;[0 0 0] Combo system
  ;;[0 0 0 0] Combo Continue
  (if (Variables|Default|GetsaveAttack)
    (Variables|Default|SetsaveAttack false)
    (switch int (Variables|Default|GetAttackIndex)
      (:0
        (CallFunction|Attack1))
      (:1
        (CallFunction|Attack2))
      (:2
        (CallFunction|Attack3))
      (:3
        (CallFunction|Attack4)))
    (else
      (CallFunction|StopCombo))))

(event Custom|StartSwordTrace
  ;[0.025 0.025 0.025] Sword Trace
  (bind _returnvalue (Utilities|Time|SetTimerbyEvent (delegate Custom|SwordTraceLoop) 0.01 true))
  (Variables|Default|SetSwordTraceLoopIndic _returnvalue))

(event Custom|StopSwordTrace
  ;[0.025 0.025 0.025] Sword Trace
  (Utilities|Time|ClearandInvalidateTimerbyHandle (Variables|Default|GetSwordTraceLoopIndic)))

(event Custom|SphericalTrace
  (bind _maincharacterbp (Variables|Default|GetMainCharacterBP))
  (bind _kick_trace (Variables|/Game/ThirdPerson/Blueprints/BP_MainCharacter.BP_MainCharacter_C|GetKick%20Trace _maincharacterbp))
  (bind _returnvalue (Transformation|GetWorldLocation _kick_trace))
  ;[0 0 0] Kick Trace and stab
  (bind (_outhit _returnvalue_2) (Collision|SphereTraceByChannel _returnvalue _returnvalue 45.0 "TraceTypeQuery1" false 0 "None"))
  (if _returnvalue_2
    (if (Actor|ActorHasTag (.HitActor (Collision|BreakHitResult _outhit)) "Damagable")
      (Game|Damage|ApplyDamage (.HitActor (Collision|BreakHitResult _outhit)) 3e+01 0 0))))

(event Custom|StopCombo
  ;[0 0 0] Combo system
  ;;[0 0 0 0] Stop Attack
  (Variables|Default|SetIsAttacking false)
  (Variables|Default|SetAttackIndex 0))

(event Custom|Attack2
  ;[0 0 0] Combo system
  ;;[0 0 0] Attack2
  (Utilities|FlowControl|DoOnce false :!label _label
    (:Completed
      (Utilities|FlowControl|Delay 0.1)
      (Animation|Montage|PlayMontage (Variables|Default|GetMainCharacterMesh) "/Game/animations/Attack2_Montage.Attack2_Montage"
        (:then
          (Variables|Default|SetAttackIndex 2)
          (goto _label Reset))))))

(event Custom|Attack1
  ;[0 0 0] Combo system
  ;;[0 0 0] Attack1
  (Utilities|FlowControl|DoOnce false :!label _label
    (:Completed
      (Utilities|FlowControl|Delay 0.1)
      (Animation|Montage|PlayMontage (Variables|Default|GetMainCharacterMesh) "/Game/animations/Attack1_Montage.Attack1_Montage"
        (:then
          (Variables|Default|SetAttackIndex 1)
          (goto _label Reset))))))

(event Custom|Attack4
  ;[0 0 0] Combo system
  ;;[0 0 0] Attack4
  (Utilities|FlowControl|DoOnce false :!label _label
    (:Completed
      (Utilities|FlowControl|Delay 0.1)
      (Animation|Montage|PlayMontage (Variables|Default|GetMainCharacterMesh) "/Game/animations/Attack3_Montage.Attack3_Montage"
        (:then
          (Variables|Default|SetAttackIndex 4)
          (goto _label Reset))))))

(event Custom|SwordTraceLoop
  ;[0.025 0.025 0.025] Sword Trace
  (bind (_outhit _returnvalue) (Collision|SphereTraceByChannel (Transformation|GetWorldLocation (Variables|/Game/ThirdPerson/Blueprints/BP_MainCharacter.BP_MainCharacter_C|GetSwordTopPoint (Variables|Default|GetMainCharacterBP))) (Transformation|GetWorldLocation (Variables|/Game/ThirdPerson/Blueprints/BP_MainCharacter.BP_MainCharacter_C|GetSwordBottomPoint1 (Variables|Default|GetMainCharacterBP))) 35.0 "TraceTypeQuery1" false 0 "None"))
  (if _returnvalue
    (if (Actor|ActorHasTag (.HitActor (Collision|BreakHitResult _outhit)) "Damagable")
      (Utilities|FlowControl|DoOnce false :!label _label
        (:Completed
          (Game|Damage|ApplyDamage (.HitActor (Collision|BreakHitResult _outhit)) 25.0 0 0)
          (Utilities|FlowControl|Delay 0.5)
          (goto _label Reset))))))

(event Custom|Attack3
  ;[0 0 0] Combo system
  ;;[0 0 0] Attack3  Kick
  (Utilities|FlowControl|DoOnce false :!label _label
    (:Completed
      (Utilities|FlowControl|Delay 0.1)
      (Animation|Montage|PlayMontage (Variables|Default|GetMainCharacterMesh) "/Game/animations/Kick_Montage.Kick_Montage"
        (:then
          (Variables|Default|SetAttackIndex 3)
          (goto _label Reset))))))

(event Input|EnhancedActionEvents|EnhancedInputActionIA_Attack
  (params (ActionValue :type Boolean) (ElapsedSeconds :type Float%20%28double-precision%29) (TriggeredSeconds :type Float%20%28double-precision%29) (InputAction :type Input%20Action%20Object%20Reference :default "/Game/ThirdPerson/Input/Actions/IA_Attack.IA_Attack"))
  (if (Variables|Default|GetCanAttack)
    (CallFunction|Attack4)
    (bind (_outhit _returnvalue) (Collision|SphereTraceByChannel (Transformation|GetWorldLocation (Variables|/Game/ThirdPerson/Blueprints/BP_MainCharacter.BP_MainCharacter_C|GetSwordTopPoint (Variables|Default|GetMainCharacterBP))) (Transformation|GetWorldLocation (Variables|/Game/ThirdPerson/Blueprints/BP_MainCharacter.BP_MainCharacter_C|GetSwordBottomPoint1 (Variables|Default|GetMainCharacterBP))) 35.0 "TraceTypeQuery1" false 0 "None"))
    (if _returnvalue
      (if (Actor|ActorHasTag (.HitActor (Collision|BreakHitResult _outhit)) "Damagable")
        (Game|Damage|ApplyDamage (.HitActor (Collision|BreakHitResult _outhit)) 25.0 0 0)))))

(event Input|EnhancedActionEvents|EnhancedInputActionIA_AttackCombo
  (params (ActionValue :type Boolean) (ElapsedSeconds :type Float%20%28double-precision%29) (TriggeredSeconds :type Float%20%28double-precision%29) (InputAction :type Input%20Action%20Object%20Reference :default "/Game/ThirdPerson/Input/Actions/IA_AttackCombo.IA_AttackCombo"))
  ;[0 0 0] Combo system
  ;;[0 0 0 0] Attack Input
  (:Started
    (if (Variables|Default|GetCanAttack)
      (CallFunction|SwordAttack))))

(event Input|EnhancedActionEvents|EnhancedInputActionIA_Kick
  (params (ActionValue :type Boolean) (ElapsedSeconds :type Float%20%28double-precision%29) (TriggeredSeconds :type Float%20%28double-precision%29) (InputAction :type Input%20Action%20Object%20Reference :default "/Game/ThirdPerson/Input/Actions/IA_Kick.IA_Kick"))
  (if (Variables|Default|GetCanAttack)
    (CallFunction|Attack3)
    (CallFunction|SphericalTrace)))

(event Input|EnhancedActionEvents|EnhancedInputActionIA_Stab
  (params (ActionValue :type Boolean) (ElapsedSeconds :type Float%20%28double-precision%29) (TriggeredSeconds :type Float%20%28double-precision%29) (InputAction :type Input%20Action%20Object%20Reference :default "/Game/ThirdPerson/Input/Actions/IA_Stab.IA_Stab"))
  (if (Variables|Default|GetCanAttack)
    (CallFunction|Attack2)
    (CallFunction|SphericalTrace)))

(event EventBeginPlay
  (bind _asbp_main_character (Utilities|Casting|CastToBP_MainCharacter (Components|GetOwner)))
  (Variables|Default|SetMainCharacterBP _asbp_main_character)
  (Variables|Default|SetMainCharacterMesh (Variables|/Script/Engine.Character|GetMesh _asbp_main_character)))