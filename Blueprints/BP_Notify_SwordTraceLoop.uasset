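; Anim notify state that marks the window in an animation during which sword hit tracing runs.
; On begin, it starts the trace through the main character's BPCAttackSystem, or directly on BP_AIWarrior if the owner is not the player character.
; On end, it stops the trace only for the main character, as the AI warrior's stop branch is never executed.
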(fn ReceivedNotifyBegin
  (params (MeshComp :type Skeletal%20Mesh%20Component%20Object%20Reference) (Animation :type Anim%20Sequence%20Base%20Object%20Reference) (TotalDuration :type Float%20%28single-precision%29) (EventReference :type Anim%20Notify%20Event%20Reference%20Structure%20%28by%20ref%29))
  (bind _returnvalue (Components|GetOwner MeshComp))
  (bind _asbp_main_character (Utilities|Casting|CastToBP_MainCharacter _returnvalue)
    (:then
      (Default|StartSwordTrace (Variables|/Game/ThirdPerson/Blueprints/BP_MainCharacter.BP_MainCharacter_C|GetBPC_AttackSystem _asbp_main_character)))
    (:CastFailed
      (bind _asbp_aiwarrior (Utilities|Casting|CastToBP_AIWarrior _returnvalue))
      (Default|StartSwordTrace _asbp_aiwarrior)))
  (return false))

(fn ReceivedNotifyEnd
  (params (MeshComp :type Skeletal%20Mesh%20Component%20Object%20Reference) (Animation :type Anim%20Sequence%20Base%20Object%20Reference) (EventReference :type Anim%20Notify%20Event%20Reference%20Structure%20%28by%20ref%29))
  (bind _asbp_main_character (Utilities|Casting|CastToBP_MainCharacter (Components|GetOwner MeshComp)))
  (Default|StopSwordTrace (Variables|/Game/ThirdPerson/Blueprints/BP_MainCharacter.BP_MainCharacter_C|GetBPC_AttackSystem _asbp_main_character))
  (return false))