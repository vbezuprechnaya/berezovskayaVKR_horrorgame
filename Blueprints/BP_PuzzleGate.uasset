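; BP_PuzzleGate is a gate that swings open once enough items have been collected.
; Each Collectiteam call increments a counter, and reaching the maximum fires OpenDoor and a 2D gate sound through a DoOnce, so both happen only once.
; OpenDoor plays a timeline that lerps the door's relative yaw from closed to partly open.
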(event Custom|OpenDoor
  (bind _door_rotation (Timeline|Open%20Door%20Anim Play)
    (:Update
      (Transformation|SetRelativeRotation (Variables|Default|Getdoor) (Math|Rotator|MakeRotator 0.0 0.0 (Math|Float|Lerp 0.0 6e+01 _door_rotation)) false false))))

(event Custom|Collectiteam
  (Math|Integer|IncrementInt (Variables|Default|GetcurrentIteamCollected)
    (:%20%20
      (if (>= (Variables|Default|GetcurrentIteamCollected) (Variables|Default|GetMaxIteamCollectable))
        (Utilities|FlowControl|DoOnce false
          (:Completed
            (CallFunction|OpenDoor)
            (Audio|PlaySound2D "/Game/audio/404068__swordofkings128__backyard-gate-open.404068__swordofkings128__backyard-gate-open" 1.0 1.0 0.0 0 0 false)))))))

(fn ConstructionScript)