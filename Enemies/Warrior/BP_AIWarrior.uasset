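; Enemy AI warrior character that fights the player with melee attacks and registers itself as an agent with tagged Learning Agents managers.
; Attack triggers a random pick of sword combo, kick, stab or alternate strike, with montages advancing a combo index.
; Capsule overlaps, looped on a timer for sword swings or one-shot for other strikes, apply damage.
; Incoming damage plays a hit reaction, or ragdolls the warrior at zero health.
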(event Custom|SwordAttack
  ;[0 0 0] Combo system
  ;;[0 0 0 0] Sword Attack
  (if (Variables|Default|GetIsAttacking)
    (Variables|Default|SetsaveAttack true)
    (else
      (Variables|Default|SetsaveAttack false)
      (switch int (Variables|Default|GetAttackIndex)
        (:0
          (CallFunction|Attack1))
        (:1
          (CallFunction|Attack2))
        (:2
          (CallFunction|Attack3))
        (:3
          (CallFunction|Attack4))))))

(event Custom|SwordAttackCombo
  ;[0 0 0] Combo system
  ;;[0 0 0 0] Combo Continue
  (if (Variables|Default|GetsaveAttack)
    (Variables|Default|SetsaveAttack false)
    (switch int (Variables|Default|GetAttackIndex)
      (:0
        (CallFunction|Attack1))
      (:1
        (CallFunction|Attack2))
      (:2
        (CallFunction|Attack3))
      (:3
        (CallFunction|Attack4)))
    (else
      (CallFunction|StopCombo))))

(event Custom|diffAttack3
  (if (Variables|Default|GetCanAttack)
    (CallFunction|Attack4)
    (bind (_outactors _returnvalue) (Collision|CapsuleOverlapActors (Transformation|GetWorldLocation (Variables|Default|GetTrigger)) (Variables|Default|GetSwordRadius) 0.0 (Utilities|Array|MakeArray "ObjectTypeQuery3") "/Game/ThirdPerson/Blueprints/BP_MainCharacter.BP_MainCharacter_C" (Utilities|Array|MakeArray 0)))
    (if _returnvalue
      (Game|Damage|ApplyDamage (.ReturnValue (Actor|FindNearestActor (Transformation|GetActorLocation (Game|Player|GetPlayerPawn 0)) _outactors)) 5.0 (Pawn|GetController) self))))

(event Custom|StartSwordTrace
  ;[0.025 0.025 0.025] Sword Trace
  (bind _returnvalue (Utilities|Time|SetTimerbyEvent (delegate Custom|SwordTraceLoop) 0.01 true))
  (Variables|Default|SetSwordTraceLoopIndic _returnvalue))

(event Custom|SwordTraceLoop
  ;[0.025 0.025 0.025] Sword Trace
  (bind (_outactors _returnvalue) (Collision|CapsuleOverlapActors (Transformation|GetWorldLocation (Variables|Default|GetTrigger)) (Variables|Default|GetSwordRadius) 0.0 (Utilities|Array|MakeArray "ObjectTypeQuery3") "/Game/ThirdPerson/Blueprints/BP_MainCharacter.BP_MainCharacter_C" (Utilities|Array|MakeArray self)))
  (if _returnvalue
    (for _array_element _outactors
      (Game|Damage|ApplyDamage _array_element 5.0 (Pawn|GetController) self)
      (Utilities|FlowControl|Delay 0.5))))

(event Custom|StopSwordTrace
  ;[0.025 0.025 0.025] Sword Trace
  (Utilities|Time|ClearandInvalidateTimerbyHandle (Variables|Default|GetSwordTraceLoopIndic)))

(event Custom|SphericalTrace
  ;[0 0 0] Kick Trace and stab
  (bind _returnvalue (Collision|CapsuleOverlapActors (Transformation|GetWorldLocation (Variables|Default|GetKick%20Trace)) 45.0 0.0 (Utilities|Array|MakeArray "ObjectTypeQuery3") "/Game/ThirdPerson/Blueprints/BP_MainCharacter.BP_MainCharacter_C" (Utilities|Array|MakeArray self)))
  (if _returnvalue
    (Game|Damage|ApplyDamage (Game|Player|GetPlayerPawn 0) 15.0 (Pawn|GetController) self)))

(event Custom|StopCombo
  ;[0 0 0] Combo system
  ;;[0 0 0 0] Stop Attack
  (Variables|Default|SetIsAttacking false)
  (Variables|Default|SetAttackIndex 0))

(event Custom|StabAttack
  (if (Variables|Default|GetCanAttack)
    (CallFunction|Attack2)
    (CallFunction|SphericalTrace)
    (Utilities|FlowControl|Delay 0.2)))

(event Custom|Attack1
  ;[0 0 0] Combo system
  ;;[0 0 0] Attack1
  (Utilities|FlowControl|DoOnce false :!label _label
    (:Completed
      (Utilities|FlowControl|Delay 0.1)
      (Animation|Montage|PlayMontage (Variables|Character|GetMesh) "/Game/animations/Attack1_Montage.Attack1_Montage"
        (:then
          (Variables|Default|SetAttackIndex 1)
          (goto _label Reset))))))

(event Custom|kickAttack
  (if (Variables|Default|GetCanAttack)
    (CallFunction|Attack3)
    (CallFunction|SphericalTrace)
    (Utilities|FlowControl|Delay 0.2)))

(event Custom|Attack4
  ;[0 0 0] Combo system
  ;;[0 0 0] Attack4
  (Utilities|FlowControl|DoOnce false :!label _label
    (:Completed
      (Utilities|FlowControl|Delay 0.1)
      (Animation|Montage|PlayMontage (Variables|Character|GetMesh) "/Game/animations/Attack3_Montage.Attack3_Montage"
        (:then
          (Variables|Default|SetAttackIndex 4)
          (goto _label Reset))))))

(event Custom|Attack2
  ;[0 0 0] Combo system
  ;;[0 0 0] Attack2
  (Utilities|FlowControl|DoOnce false :!label _label
    (:Completed
      (Utilities|FlowControl|Delay 0.1)
      (Animation|Montage|PlayMontage (Variables|Character|GetMesh) "/Game/animations/Attack2_Montage.Attack2_Montage"
        (:then
          (Variables|Default|SetAttackIndex 2)
          (goto _label Reset))))))

(event Custom|SwordAttackByBT
  ;[0 0 0] Combo system
  ;;[0 0 0 0] Attack Input
  (bind _output_get (Variables|Default|SetSelection (Math|Random|RandomInteger 4)))
  (if (Variables|Default|GetCanAttack)
    (switch int _output_get
      (:0
        (CallFunction|SwordAttack))
      (:1
        (CallFunction|KickAttack))
      (:2
        (CallFunction|StabAttack))
      (:3
        (CallFunction|DiffAttack3)))))

(event Custom|Attack3
  ;[0 0 0] Combo system
  ;;[0 0 0] Attack3  Kick
  (Utilities|FlowControl|DoOnce false :!label _label
    (:Completed
      (Utilities|FlowControl|Delay 0.1)
      (Animation|Montage|PlayMontage (Variables|Character|GetMesh) "/Game/animations/Kick_Montage.Kick_Montage"
        (:then
          (Variables|Default|SetAttackIndex 3)
          (goto _label Reset))))))

(event EventBeginPlay
  (Utilities|FlowControl|Sequence
    (:then_0
      (bind _outactors (Actor|GetAllActorsOfClass "BP_AIWarrior_C"))
      (Variables|Default|SetEnemies _outactors))
    (:then_1
      (bind _outactors_2 (Actor|GetAllActorswithTag "LearningAgentWar"))
      (for _array_element _outactors_2
        (Utilities|IsValid (Actor|GetComponentbyClass _array_element "/Script/LearningAgents.LearningAgentsManager")
          (:Is%20Valid
            (bind _returnvalue (Class|LearningAgentsManager|AddAgent (Actor|GetComponentbyClass _array_element "/Script/LearningAgents.LearningAgentsManager") self))
            (bind _output_get (Variables|Default|SetAgentID _returnvalue))
            (Development|PrintString (Utilities|String|Append "Agent" (Utilities|String|ToString(Integer) _output_get)) true true "(R=0.000000,G=0.660000,B=1.000000,A=1.000000)" 5.0))))
      (Development|PrintString "All set " true true "(R=1.000000,G=0.234048,B=0.061898,A=1.000000)"))))

(event Game|Damage|EventAnyDamage
  (params (Damage :type Float%20%28single-precision%29) (DamageType :type Damage%20Type%20Object%20Reference) (InstigatedBy :type Controller%20Object%20Reference) (DamageCauser :type Actor%20Object%20Reference))
  (Variables|Default|SetHealthW (- (Variables|Default|GetHealthW) Damage))
  (if (<= (Variables|Default|GetHealthW) 0.0)
    (Collision|SetCollisionObjectType (Variables|Character|GetMesh) "ECC_PhysicsBody")
    (Physics|SetSimulatePhysics (Variables|Character|GetMesh) true)
    (Pawn|Components|CharacterMovement|SetMovementMode (Variables|Character|GetCharacterMovement) "MOVE_None" 0)
    (Variables|Default|SetIsAlive false)
    (else
      (Animation|PlayAnimMontage "/Game/animations/HitReact_Left_Montage.HitReact_Left_Montage" 1.0 "None"))))

(fn ConstructionScript)

(fn Attack
  (CallFunction|SwordAttackbyBT)
  (return 0.4))